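; BP_Battery is a collectible battery actor that gives power to the player character.
; On BeginPlay it rolls rounded random Power and LifeTime values within its min and max ranges, though LifeTime is not used further in this graph.
; The Collected event casts player 0 to BatteryManCharacter, adds Power to its StoredPower, prints debug text and destroys the battery.
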(event `self.ReceiveBeginPlay`
  (set `self.Power` (`KismetMathLibrary.Conv_IntToDouble` (`KismetMathLibrary.Round` (`KismetMathLibrary.RandomFloatInRange` (`self.PowerMin`) (`self.PowerMax`)))))
  (set `self.LifeTime` (`KismetMathLibrary.Conv_IntToDouble` (`KismetMathLibrary.Round` (`KismetMathLibrary.RandomFloatInRange` (`self.LifeTimeMin`) (`self.LifeTimeMax`))))))

(event `self.Collected`
  (`KismetSystemLibrary.PrintString` "Collected")
  (bind _asbattery_man_character (cast `BatteryManCharacter` (`GameplayStatics.GetPlayerCharacter` 0)))
  (bind _output_get (set `BatteryManCharacter.StoredPower` (+ (`BatteryManCharacter.StoredPower` _asbattery_man_character) (`self.Power`)) _asbattery_man_character))
  (`KismetSystemLibrary.PrintString` (`KismetStringLibrary.Conv_DoubleToString` _output_get))
  (`self.K2_DestroyActor`))

(fn `UserConstructionScript`)