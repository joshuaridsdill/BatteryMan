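; BP_Powered_Battery is a collectible battery variant built as a child Blueprint of a parent class not named here.
; On BeginPlay it sets its minimum and maximum power and lifetime ranges, then calls the parent's BeginPlay.
; The Collected event and construction script only forward to the parent, and overlap and Tick are disabled stubs.
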(event `self.ReceiveBeginPlay`
  (set `self.PowerMin` 40.0)
  (set `self.PowerMax` 60.0)
  (set `self.LifeTimeMin` 2.0)
  (set `self.LifeTimeMax` 5.0)
  (`parent.ReceiveBeginPlay`))

(event `self.Collected`
  (`parent.Collected`))

(fn `UserConstructionScript`
  (`parent.UserConstructionScript`))